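; Game mode that runs an endless wave-based zombie survival loop with a warning widget between waves.
; Each wave shows the warning for a short delay, then spawns three BP_Zombie per wave number at SpawnLocation, adjusting for collisions.
; EnemyKilled decrements the remaining count and, at zero, increments the wave and repeats the warning and spawn.
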(event Custom|Start%20Game
  (Utilities|FlowControl|Delay 5.0)
  (Widget|SetVisibility (Variables|Default|GetWaveWarningUI) "Hidden")
  (CallFunction|SpawnEnemies))

(event Custom|Spawn%20Enemies
  (bind _output_get (Variables|Default|SetTotal%20Enemies (* (Variables|Default|GetCurrent%20Wave) 3)))
  (Variables|Default|SetRemaining%20Enemies _output_get)
  (bind _index (Utilities|FlowControl|ForLoopwithBreak 0 _output_get :!label _label)
    (:LoopBody
      (if (!= _index (Variables|Default|GetTotal%20Enemies))
        (Game|SpawnActorfromClass "/Game/Characters/Zombie/BP_Zombie.BP_Zombie_C" (Variables|Default|GetSpawn%20Location) "AdjustIfPossibleButAlwaysSpawn" "MultiplyWithRoot" 0 0)
        (else
          (goto _label Break))))))

(event Custom|Enemy%20Killed
  (bind _result (Math|Integer|DecrementInt (Variables|Default|GetRemaining%20Enemies))
    (:%20%20
      (if (== _result 0)
        (CallFunction|WaveIncrement)))))

(event Custom|Wave%20Increment
  (bind _wavewarningui (Variables|Default|GetWaveWarningUI))
  (Math|Integer|IncrementInt (Variables|Default|GetCurrent%20Wave)
    (:%20%20
      (Widget|SetVisibility _wavewarningui "Visible")
      (Utilities|FlowControl|Delay 5.0)
      (Widget|SetVisibility _wavewarningui "Hidden")
      (CallFunction|SpawnEnemies))))

(event EventBeginPlay
  (bind _returnvalue (UserInterface|CreateWidget "/Game/_main/HUD/UI_WaveWarning.UI_WaveWarning_C"))
  (bind _output_get (Variables|Default|SetWaveWarningUI _returnvalue))
  (UserInterface|Viewport|AddtoViewport _output_get 0)
  (CallFunction|StartGame))

(fn ConstructionScript)